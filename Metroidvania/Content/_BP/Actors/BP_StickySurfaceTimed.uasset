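; BP_StickySurfaceTimed is a surface actor that temporarily changes the speed of actors overlapping it.
; On begin overlap it applies SpeedModifier through PawnSpeed_Interface to any actor implementing it.
; After a LifeSpan delay started by that overlap, it restores the actor's speed and destroys itself.
; Leaving the surface does not restore speed, as EndOverlap is empty and its restore logic is disconnected.
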(event `self.ReceiveActorBeginOverlap`
  (params (OtherActor :type "Actor Object Reference"))
  (if (`KismetSystemLibrary.DoesImplementInterface` OtherActor "/Game/_BP/Interface/PawnSpeed_Interface.PawnSpeed_Interface_C")
    (message `/Game/_BP/Interface/PawnSpeed_Interface.ModifyPawnSpeed` OtherActor (`self.SpeedModifier`))
    (`KismetSystemLibrary.Delay` (`self.LifeSpan`))
    (message `/Game/_BP/Interface/PawnSpeed_Interface.RestorePawnSpeed` OtherActor)
    (`self.K2_DestroyActor`)))

(event `self.ReceiveActorEndOverlap`
  (params (OtherActor :type "Actor Object Reference")))

(fn `UserConstructionScript`)