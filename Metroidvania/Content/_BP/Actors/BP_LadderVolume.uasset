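; BP_LadderVolume is a box trigger that marks a climbable area for BP_PlayerCharacter.
; On overlap begin it sets the character's CanClimb flag and multiplies its MaxFlySpeed by SpeedModifier.
; On overlap end it clears the flag, restores Walking movement and divides MaxFlySpeed by SpeedModifier, using the character reference cast in the begin event.
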(event `self.Box.OnComponentBeginOverlap`
  (params (OverlappedComponent :type "PrimitiveComponent Object Reference") (OtherActor :type "Actor Object Reference") (OtherComp :type "PrimitiveComponent Object Reference") (OtherBodyIndex :type Integer) (bFromSweep :type Boolean) (SweepResult :type "HitResult Structure (by ref)"))
  (bind _asbp_player_character (cast `/Game/_BP/BP_PlayerCharacter` OtherActor))
  (set `/Game/_BP/BP_PlayerCharacter.CanClimb` true _asbp_player_character)
  (bind _charactermovement (`Character.CharacterMovement` _asbp_player_character))
  (set `CharacterMovementComponent.MaxFlySpeed` (* (`CharacterMovementComponent.MaxFlySpeed` _charactermovement) (`self.SpeedModifier`)) _charactermovement))

(event `self.Box.OnComponentEndOverlap`
  (params (OverlappedComponent :type "PrimitiveComponent Object Reference") (OtherActor :type "Actor Object Reference") (OtherComp :type "PrimitiveComponent Object Reference") (OtherBodyIndex :type Integer))
  (bind _asbp_player_character (cast `/Game/_BP/BP_PlayerCharacter` OtherActor))
  (set `/Game/_BP/BP_PlayerCharacter.CanClimb` false _asbp_player_character)
  (`CharacterMovementComponent.SetMovementMode` (`Character.CharacterMovement` _asbp_player_character) "MOVE_Walking" 0)
  (bind _charactermovement (`Character.CharacterMovement` (stale `self.Box.OnComponentBeginOverlap` _asbp_player_character)))
  (set `CharacterMovementComponent.MaxFlySpeed` (/ (`CharacterMovementComponent.MaxFlySpeed` _charactermovement) (`self.SpeedModifier`)) _charactermovement))

(fn `UserConstructionScript`)