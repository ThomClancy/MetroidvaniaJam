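; BP_StickyGrenade is a grenade actor that leaves a timed sticky surface behind on contact.
; On any actor overlap it spawns BP_StickySurfaceTimed at the other actor's transform, destroys itself, then sets HitPawn.
; BeginPlay and Destroyed are empty, while logic for a lifespan and a fallback surface at the grenade's own position when HitPawn is false sits disconnected and never runs.
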(event `self.ReceiveBeginPlay`)

(event `self.ReceiveActorBeginOverlap`
  (params (OtherActor :type "Actor Object Reference"))
  (`|SpawnActorFromClass` "/Game/_BP/Actors/BP_StickySurfaceTimed.BP_StickySurfaceTimed_C" (`self.GetTransform` OtherActor) "AlwaysSpawn" "OverrideRootScale" null null)
  (`self.K2_DestroyActor`)
  (set `self.HitPawn` true))

(event `self.ReceiveDestroyed`)

(fn `UserConstructionScript`)