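; Grappling hook projectile that either launches the player to a zip line point or pulls grapple objects back.
; On hit, zip line actors trigger a player launch when CanGrappleToLocation is set; otherwise timelines lerp the hook and any BP_GrappleObject to the hook's spawn location.
; GrapplingHookRange acts as a delay before automatic retraction.
; The hook re-enables the player's CanZip after launching, or upon destroying itself when retraction finishes.
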(event `self.Sphere1.OnComponentHit`
  (params (HitComponent :type "PrimitiveComponent Object Reference") (OtherActor :type "Actor Object Reference") (OtherComp :type "PrimitiveComponent Object Reference") (NormalImpulse :type "Vector Structure") (Hit :type "HitResult Structure (by ref)"))
  (bind _returnvalue (`GameplayStatics.GetPlayerCharacter` 0))
  ;[1 1 1] Are we going TO and object or PULLING an object to us?
  (if (`self.CanGrappleToLocation`)
    (if (`KismetSystemLibrary.DoesImplementInterface` OtherActor "/Game/_BP/Interface/ZipLine_Interface.ZipLine_Interface_C")
      ;[1 1 1] Launch Player to Grapple Point
      (bind _asbp_zip_line_point (cast `/Game/_BP/Actors/BP_ZipLinePoint` OtherActor))
      (bind _asbp_player_character (cast `/Game/_BP/BP_PlayerCharacter` _returnvalue))
      (`Character.LaunchCharacter` _returnvalue (0.0 0.0 500.0) true true)
      (`Character.LaunchCharacter` _asbp_player_character (0.0 0.0 500.0) true true)
      (`Character.LaunchCharacter` _returnvalue (* (- (`SceneComponent.K2_GetComponentLocation` (`/Game/_BP/Actors/BP_ZipLinePoint.ZipLinePoint` _asbp_zip_line_point)) (`self.K2_GetActorLocation` _returnvalue)) 2.5) true true)
      (bind _asbp_player_character_2 (cast `/Game/_BP/BP_PlayerCharacter` (`GameplayStatics.GetPlayerCharacter` 0)))
      (set `/Game/_BP/BP_PlayerCharacter.CanZip` true _asbp_player_character_2)
      (else
        (`|ExecutionSequence` :!label _label
          (:`then_0`
            ;[1 1 1] Launch and Return Grappling Hook
            (bind (_direction _lerpalpha) (`Timeline|ReturnToPlayer` :!label _label_2)
              (:`Update`
                (set `MovementComponent.Velocity` (0.0 0.0 0.0) (`self.ProjectileMovement`))
                (`SceneComponent.K2_SetWorldLocation` (`self.Sphere1`) (`KismetMathLibrary.VLerp` (`SceneComponent.K2_GetComponentLocation` (`self.Sphere1`)) (stale `self.ReceiveBeginPlay` _output_get) _lerpalpha) false false))
              (:`Finished`
                (`self.K2_DestroyActor`)
                ;[1 1 1] Return player's ability to throw grappling hook
                (bind _asbp_player_character_3 (cast `/Game/_BP/BP_PlayerCharacter` (`GameplayStatics.GetPlayerCharacter` 0) :!label _label_3))
                (set `/Game/_BP/BP_PlayerCharacter.CanZip` true _asbp_player_character_3))))
          (:`then_1`
            ;[1 1 1] Pull Object back to Player
            (bind _asbp_grapple_object (cast `/Game/_BP/Actors/BP_GrappleObject` OtherActor))
            (bind (_direction_2 _lerpalpha_2) (`Timeline|Timeline_0`)
              (:`Update`
                (bind _capsule (`/Game/_BP/Actors/BP_GrappleObject.Capsule` _asbp_grapple_object))
                (`SceneComponent.K2_SetWorldLocation` _capsule (`KismetMathLibrary.VLerp` (`SceneComponent.K2_GetComponentLocation` _capsule) (`self.SpawnLocation`) _lerpalpha_2) false false))
              (:`Finished`
                (`self.K2_DestroyActor`)
                (goto _label_3)))))))
    (else
      (goto _label))))

(event `self.ReceiveBeginPlay`
  ;[1 1 1] Initial Set Up
  (bind _output_get (set `self.SpawnLocation` (`SceneComponent.K2_GetComponentLocation` (`self.Sphere1`))))
  (`KismetSystemLibrary.Delay` (`self.GrapplingHookRange`))
  (goto _label_2))

(fn `UserConstructionScript`)