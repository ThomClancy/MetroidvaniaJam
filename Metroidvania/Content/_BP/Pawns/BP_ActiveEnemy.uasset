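; BP_ActiveEnemy is an enemy pawn that takes projectile damage and spawns a pickup at its capsule's location when it dies.
; ProjectileDamage feeds UpdateHealth, which adds the incoming value to health, so damage must be negative, and destroys the actor at zero or below.
; UpdateSpeed multiplies the current walk speed, so modifiers stack until RestoreSpeed reapplies BaseMovementSpeed.
; The sight-sensing handler is empty.
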(event `self.ReceiveBeginPlay`
  (set `self.BaseMovementSpeed` (`self.BaseMovementSpeed`)))

(event `self.PawnSensing.OnSeePawn`
  (params (Pawn :type "Pawn Object Reference")))

(event `/Game/_BP/Interface/Projectile_Interface.ReceiveProjectileDamage`
  (params (IncomingDamage :type "Float (single-precision)"))
  ;[1 1 1] Take Damage
  (`self.UpdateHealth` IncomingDamage (`self.PickUpToSpawn`)))

(fn `RestoreSpeed`
  (set `CharacterMovementComponent.MaxWalkSpeed` (`self.BaseMovementSpeed`) (`self.CharacterMovement`)))

(fn `UpdateHealth`
  (params (IncomingDamage :type "Float (double-precision)") (IncomingPickup :type "Actor Class Reference"))
  (bind _output_get (set `self.PawnHealth` (+ IncomingDamage (`self.PawnHealth`))))
  (if (<= _output_get 0.0)
    (`|SpawnActorFromClass` IncomingPickup (`KismetMathLibrary.Conv_VectorToTransform` (`SceneComponent.K2_GetComponentLocation` (`self.CapsuleComponent`))) "AlwaysSpawn" "OverrideRootScale" null null)
    (`self.K2_DestroyActor`)))

(fn `UpdateSpeed`
  (params (SpeedModifier :type "Float (double-precision)"))
  (bind _charactermovement (`self.CharacterMovement`))
  (set `CharacterMovementComponent.MaxWalkSpeed` (* SpeedModifier (`CharacterMovementComponent.MaxWalkSpeed` _charactermovement)) _charactermovement))

(fn `UserConstructionScript`)