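; Passive enemy pawn that moves toward the player on sight, deals damage on contact and drops a pickup when killed.
; PawnSensing triggers an AI MoveTo, whose immediate exec output switches movement off for a second before restoring walking.
; DamageBox overlap sends PawnDamage through Projectile_Interface; the logic to limit repeat damage is unfinished.
; Incoming damage is added to health, and at or below DeadHealth the pawn destroys itself and spawns its pickup.
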(event `self.PawnSensing.OnSeePawn`
  (params (Pawn :type "Pawn Object Reference"))
  (bind _charactermovement (`self.CharacterMovement`))
  ;[1 1 1] I think this will stop the pawn for a second after they reach the player
  (bind _asbp_player_character (cast `/Game/_BP/BP_PlayerCharacter` Pawn))
  (bind _movementresult (`|AIMoveTo` self (0.0 0.0 0.0) _asbp_player_character)
    (:`then`
      (`CharacterMovementComponent.SetMovementMode` _charactermovement "MOVE_None" _movementresult)
      (`KismetSystemLibrary.Delay` 1.0)
      (`CharacterMovementComponent.SetMovementMode` _charactermovement "MOVE_Walking" 0))))

(event `self.DamageBox.OnComponentBeginOverlap`
  (params (OverlappedComponent :type "PrimitiveComponent Object Reference") (OtherActor :type "Actor Object Reference") (OtherComp :type "PrimitiveComponent Object Reference") (OtherBodyIndex :type Integer) (bFromSweep :type Boolean) (SweepResult :type "HitResult Structure (by ref)"))
  ;[1 1 1] Base damage logic - send damage to player when they overlap with collision box
  (if (`KismetSystemLibrary.DoesImplementInterface` OtherActor "/Game/_BP/Interface/Projectile_Interface.Projectile_Interface_C")
    (message `/Game/_BP/Interface/Projectile_Interface.ReceiveProjectileDamage` OtherActor (`self.PawnDamage`))))

(event `self.DamageBox.OnComponentEndOverlap`
  (params (OverlappedComponent :type "PrimitiveComponent Object Reference") (OtherActor :type "Actor Object Reference") (OtherComp :type "PrimitiveComponent Object Reference") (OtherBodyIndex :type Integer))
  ;[1 1 1] Trying to set it up so that damage doesn't continue to rack up while overlapped with player
)

(event `/Game/_BP/Interface/Projectile_Interface.ReceiveProjectileDamage`
  (params (IncomingDamage :type "Float (single-precision)"))
  ;[1 1 1] Receive Damage
  (`self.UpdateHealth` IncomingDamage (`self.PickUpToSpawn`)))

(fn `UpdateHealth`
  (params (IncomingDamage :type "Float (double-precision)") (IncomingPickup :type "Actor Class Reference"))
  (bind _output_get (set `self.PawnHealth` (+ (`self.PawnHealth`) IncomingDamage)))
  (`/Engine/EditorBlueprintResources/StandardMacros.CompareFloat` _output_get (`self.DeadHealth`)
    (:`==`
      _)
    (:`<`
      _))
  (`self.K2_DestroyActor`)
  (`|SpawnActorFromClass` IncomingPickup (`KismetMathLibrary.Conv_VectorToTransform` (`SceneComponent.K2_GetComponentLocation` (`self.Cube`))) "Undefined" "OverrideRootScale" null null))

(fn `UserConstructionScript`)