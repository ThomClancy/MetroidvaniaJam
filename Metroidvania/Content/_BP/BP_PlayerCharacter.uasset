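; Player character Blueprint handling movement, look, jumping, prototype wall climbing, projectile shooting, sticky grenades and health.
; CanClimb switches forward input to flying movement along the up vector and turns jumps into backward launches.
; Zip line traces for ZipLine_Interface actors, animates a rope, then launches toward the hit with briefly reduced gravity and a cooldown.
; Incoming damage adjusts clamped health, destroying the actor at the death threshold.
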(event `InputAxis|MoveForward`
  (params (AxisValue :type "Float (single-precision)"))
  ;[1 1 1] Movement
  ;[1 1 1] First Pass Wall Walking
  (if (`self.CanClimb`)
    (`CharacterMovementComponent.SetMovementMode` (`self.CharacterMovement`) "MOVE_Flying" 0)
    (`self.AddMovementInput` (`self.GetActorUpVector` (`GameplayStatics.GetPlayerCharacter` 0)) AxisValue)
    (else
      (`self.AddMovementInput` (`KismetMathLibrary.GetForwardVector` (`self.GetControlRotation`)) AxisValue))))

(event `InputAxis|MoveRight`
  (params (AxisValue :type "Float (single-precision)"))
  ;[1 1 1] Movement
  (`self.AddMovementInput` (`KismetMathLibrary.GetRightVector` (`self.GetControlRotation`)) AxisValue))

(event `self.ReceiveBeginPlay`)

(event `InputAction|Jump`
  (params (Key :type "Key Structure"))
  ;[1 1 1] Less Rough Jump - Add another branch to see if player is climbing
  (:`Pressed`
    (if (`NavMovementComponent.IsFalling` (`self.CharacterMovement`))
      _
      (elif (`self.CanClimb`)
        ;[1 1 1] Rough jump away from wall - Currently set for forward vector, should be just away from nearest surface if possible
        (`self.LaunchCharacter` (* (`self.GetActorForwardVector`) (* (`self.JumpForce`) -1.0)) true true)
        (else
          (`self.LaunchCharacter` (`KismetMathLibrary.MakeVector` 0.0 0.0 (`self.JumpForce`))))))))

(event `InputAxis|TurnRight`
  (params (AxisValue :type "Float (single-precision)"))
  ;[1 1 1] Look Right/Left
  (`self.AddControllerYawInput` (* AxisValue (`self.BaseLookRate`) (`GameplayStatics.GetWorldDeltaSeconds`))))

(event `InputAxis|LookUpRate`
  (params (AxisValue :type "Float (single-precision)"))
  ;[1 1 1] Look Up - Fixed by using pawn rotation with Spring Arm
  (`self.AddControllerPitchInput` (* AxisValue (`self.BaseLookRate`) (`GameplayStatics.GetWorldDeltaSeconds`))))

(event `InputAction|Shoot`
  (params (Key :type "Key Structure"))
  ;[1 1 1] Super Rough Shoot
  (:`Pressed`
    (`|SpawnActorFromClass` "/Game/_BP/Actors/BP_Projectile.BP_Projectile_C" (`SceneComponent.K2_GetComponentToWorld` (`self.ProjectileSpawn`)) "Undefined" "OverrideRootScale" null null)))

(event `InputAction|ZipLine`
  (params (Key :type "Key Structure"))
  (bind _returnvalue (`self.K2_GetActorLocation`))
  (bind _charactermovement (`self.CharacterMovement`))
  ;[1 1 1] Zip Line!
  (:`Pressed`
    (if (`self.CanZip`)
      (set `self.CanZip` false)
      (bind (_outhit _returnvalue_2) (`KismetSystemLibrary.LineTraceSingle` :`Start` _returnvalue :`End` (+ _returnvalue (* (`SceneComponent.GetForwardVector` (`self.ProjectileSpawn`)) (`self.ZipDistance`))) :`TraceChannel` "TraceTypeQuery1" :`DrawDebugType` "ForDuration"))
      (if _returnvalue_2
        (bind (_bblockinghit _binitialoverlap _time _distance _location _impactpoint _normal _impactnormal _physmat _hitactor) (`GameplayStatics.BreakHitResult` _outhit))
        (set `self.ZipLineTarget` _location)
        (if (`KismetSystemLibrary.DoesImplementInterface` _hitactor "/Game/_BP/Interface/ZipLine_Interface.ZipLine_Interface_C")
          (`self.ZipLine`)
          (`self.LaunchCharacter` (0.0 0.0 200.0) true true)
          (`KismetSystemLibrary.Delay` 0.2)
          (`self.LaunchCharacter` (* (- (`self.ZipLineTarget`) (`self.K2_GetActorLocation`)) 2.5) true true)
          (`self.ResetZipLine`)
          (bind _output_get (set `CharacterMovementComponent.GravityScale` 0.5 _charactermovement))
          (`KismetSystemLibrary.Delay` _output_get)
          (set `CharacterMovementComponent.GravityScale` 1.0 _charactermovement)
          (else
            (set `self.CanZip` true :!label _label)))
        (else
          (goto _label))))))

(event `ResetZipLine`
  ;[1 1 1] Zip Line Reset
  (`SceneComponent.SetVisibility` (`self.ZipLineRope`) false false)
  (`KismetSystemLibrary.Delay` (`self.ZipLineCooldown`))
  (set `self.CanZip` true))

(event `ZipLine`
  (bind _ziplinerope (`self.ZipLineRope`))
  ;[1 1 1] Shoot visible zip line
  (`SceneComponent.SetVisibility` _ziplinerope true false)
  (bind (_direction _interpspeed) (`Timeline|ZipLineInterp` :!via `PlayFromStart`)
    (:`Update`
      (`SceneComponent.K2_SetWorldLocation` _ziplinerope (`KismetMathLibrary.VInterpTo` (`SceneComponent.K2_GetComponentLocation` _ziplinerope) (`self.ZipLineTarget`) (`self.DeltaTime`) _interpspeed) false false))))

(event `/Game/_BP/Interface/Projectile_Interface.ReceiveProjectileDamage`
  (params (IncomingDamage :type "Float (single-precision)"))
  ;[1 1 1] Receive damage
  (`self.UpdateHealth` IncomingDamage))

(event `Key|Gamepad_FaceButton_Top`
  (params (Key :type "Key Structure"))
  (bind _grenadecount (`self.GrenadeCount`))
  ;[1 1 1] Throw Grenade
  (:`Pressed`
    (`/Engine/EditorBlueprintResources/StandardMacros.CompareInt` _grenadecount
      (:`>`
        (`|SpawnActorFromClass` "/Game/_BP/Actors/BP_StickyGrenade.BP_StickyGrenade_C" (`SceneComponent.K2_GetComponentToWorld` (`self.ProjectileSpawn`)) "Undefined" "OverrideRootScale" null null)
        (`/Engine/EditorBlueprintResources/StandardMacros.DecrementInt` _grenadecount)))))

(fn `UpdateGrenade`
  (bind _result (`/Engine/EditorBlueprintResources/StandardMacros.IncrementInt` (`self.GrenadeCount`))
    (:`  `
      (set `self.GrenadeCount` _result))))

(fn `UpdateHealth`
  (params (IncomingDamage :type "Float (double-precision)"))
  (bind _output_get (set `self.PlayerHealth` (`KismetMathLibrary.FClamp` (+ (`self.PlayerHealth`) IncomingDamage) 0.0 100.0)))
  (`/Engine/EditorBlueprintResources/StandardMacros.CompareFloat` _output_get (`self.DeadHealth`)
    (:`==`
      _)
    (:`<`
      _))
  (`self.K2_DestroyActor`)
  (return))

(fn `UserConstructionScript`)